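; Player character for Aloy, with Enhanced Input movement and look, bow aiming and shooting, and an exit to the main menu.
; Aiming switches rotation to follow the controller, shows a reticle widget and plays a camera zoom timeline.
; Drawing while aiming uses timelines to animate bow, body, decoy arrow and reticle bars.
; Releasing traces from the camera and spawns an arrow projectile at FirePoint toward the hit, with rotation offsets.
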(event `self.ReceiveBeginPlay`
  ; cast to player controller for inputs
  (bind _asbp_player_controller (cast `/Game/Blueprints/BP_PlayerController` (`GameplayStatics.GetPlayerController` 0)))
  (bind _output_get (set `self.As BP Player Controller` _asbp_player_controller))
  (bind _returnvalue (pcsubsystem `EnhancedInputLocalPlayerSubsystem` _output_get))
  (`/Engine/EditorBlueprintResources/StandardMacros.IsValid` _returnvalue
    (:`Is Valid`
      ;; adds inputs and sets start states and visibility
      (`EnhancedInputSubsystemInterface.AddMappingContext` _returnvalue "/Game/Inputs/IMC_MouseControls.IMC_MouseControls" 0 (struct))
      (set `self.IsAiming` false)
      (set `self.bowDrawn` false)
      (`SceneComponent.SetVisibility` (`self.ArrowDecoy`) false false)
      (`SceneComponent.SetVisibility` (`self.reticleBars1`) false false)
      (`SceneComponent.SetVisibility` (`self.reticleBars`) false false))))

(event `EnhancedInput|/Game/Inputs/Actions/IA_Aim`
  (params (ActionValue :type Boolean) (ElapsedSeconds :type "Float (double-precision)") (TriggeredSeconds :type "Float (double-precision)") (InputAction :type "InputAction Object Reference" :default "/Game/Inputs/Actions/IA_Aim.IA_Aim"))
  (bind _springarm (`self.SpringArm`))
  (bind _charactermovement (`self.CharacterMovement`))
  (bind _charactermovement_2 (`self.CharacterMovement`))
  (bind _socketoffset_x (`KismetMathLibrary.BreakVector` (`SpringArmComponent.SocketOffset` _springarm)))
  ; bow readied and camera zoom in for draw
  (:`Started`
    ;; changes camera movement settings when camera is zoomed in
    (set `CharacterMovementComponent.bOrientRotationToMovement` false _charactermovement)
    (set `CharacterMovementComponent.bUseControllerDesiredRotation` true _charactermovement_2)
    (set `self.IsAiming` true)
    ;; adds/removes reticle when in/out of aiming state
    (bind _returnvalue (`|CreateWidget` "/Game/Blueprints/UI/WB_Reticle.WB_Reticle_C"))
    (`UserWidget.AddToViewport` _returnvalue 0)
    (bind (_direction _arm_length) (`Timeline|Aim Zoom` :!label _label)
      (:`Update`
        ;; zooms in camera
        (set `SpringArmComponent.TargetArmLength` (`KismetMathLibrary.Lerp` (`self.armLength`) (`self.newArmLength`) _arm_length) (`self.SpringArm`))
        (set `SpringArmComponent.SocketOffset` (`KismetMathLibrary.MakeVector` _socketoffset_x (`KismetMathLibrary.Lerp` (`self.offsetY`) (`self.newOffsetY`) _arm_length) (`KismetMathLibrary.Lerp` (`self.offsetZ`) (`self.newOffsetZ`) _arm_length)) _springarm)
        ;; readies bow
        (`SceneComponent.K2_SetRelativeRotation` (`self.Bow`) (`KismetMathLibrary.MakeRotator` 0.0 0.0 (`KismetMathLibrary.Lerp` 0.0 (`self.bowReadyRot`) _arm_length)) false false))))
  (:`Completed`
    (set `CharacterMovementComponent.bOrientRotationToMovement` true _charactermovement)
    (set `CharacterMovementComponent.bUseControllerDesiredRotation` false _charactermovement_2)
    (set `self.IsAiming` false)
    (set `self.bowDrawn` false)
    (`/Engine/EditorBlueprintResources/StandardMacros.IsValid` _returnvalue
      (:`Is Valid`
        (`Widget.RemoveFromParent` _returnvalue)
        (goto _label :!via `ReverseFromEnd`))
      (:`Is Not Valid`
        (`KismetSystemLibrary.PrintString` "cant remove")))))

(event `EnhancedInput|/Game/Inputs/Actions/IA_Look`
  (params (ActionValue :type "Vector2D Structure") (ElapsedSeconds :type "Float (double-precision)") (TriggeredSeconds :type "Float (double-precision)") (InputAction :type "InputAction Object Reference" :default "/Game/Inputs/Actions/IA_Look.IA_Look"))
  ; camera move
  (:`Triggered`
    (`self.AddControllerYawInput` ActionValue_X)
    (`self.AddControllerPitchInput` ActionValue_Y)))

(event `EnhancedInput|/Game/Inputs/Actions/IA_Movement`
  (params (ActionValue :type "Vector2D Structure") (ElapsedSeconds :type "Float (double-precision)") (TriggeredSeconds :type "Float (double-precision)") (InputAction :type "InputAction Object Reference" :default "/Game/Inputs/Actions/IA_Movement.IA_Movement"))
  (bind (_returnvalue_roll _returnvalue_pitch _returnvalue_yaw) (`KismetMathLibrary.BreakRotator` (`self.GetControlRotation`)))
  ; player move
  (:`Triggered`
    (`self.AddMovementInput` (`KismetMathLibrary.GetRightVector` (`KismetMathLibrary.MakeRotator` _returnvalue_roll 0.0 _returnvalue_yaw)) ActionValue_X)
    (`self.AddMovementInput` (`KismetMathLibrary.GetForwardVector` (`KismetMathLibrary.MakeRotator` 0.0 0.0 _returnvalue_yaw)) ActionValue_Y)))

(event `EnhancedInput|/Game/Inputs/Actions/IA_Escape`
  (params (ActionValue :type Boolean) (ElapsedSeconds :type "Float (double-precision)") (TriggeredSeconds :type "Float (double-precision)") (InputAction :type "InputAction Object Reference" :default "/Game/Inputs/Actions/IA_Escape.IA_Escape"))
  ; back to main menu
  (:`Triggered`
    (`GameplayStatics.OpenLevelBySoftObjectPtr` "/Game/Levels/MainMenu.MainMenu")))

(event `EnhancedInput|/Game/Inputs/Actions/IA_DrawBow`
  (params (ActionValue :type Boolean) (ElapsedSeconds :type "Float (double-precision)") (TriggeredSeconds :type "Float (double-precision)") (InputAction :type "InputAction Object Reference" :default "/Game/Inputs/Actions/IA_DrawBow.IA_DrawBow"))
  ; draws bow in timeline, looses arrow at the end
  (:`Triggered`
    ;; if bow is aiming and drawn, shoot arrow
    (if (`self.IsAiming`)
      (set `self.bowDrawn` true)
      ;; rotates bow when readied
      (bind (_direction _bow_draw) (`Timeline|BowDraw` :!label _label_2)
        (:`Update`
          (bind _returnvalue (`KismetMathLibrary.Lerp` 0.0 (`self.bowDrawRotZ`) _bow_draw))
          (`SceneComponent.K2_SetRelativeRotation` (`self.Bow`) (`KismetMathLibrary.MakeRotator` 0.0 _returnvalue) false false)
          ;; rotates aloy's body and rotates bow to draw
          (`SceneComponent.K2_SetRelativeRotation` (`self.MeshAloy`) (`KismetMathLibrary.MakeRotator` 0.0 0.0 _returnvalue) false false)
          (`SceneComponent.K2_SetRelativeLocation` (`self.Bow`) (`KismetMathLibrary.MakeVector` (`KismetMathLibrary.Lerp` 0.0 (`self.bowReadyPosX`) _bow_draw) (`KismetMathLibrary.Lerp` 0.0 (`self.bowDrawPosY`) _bow_draw)) false false)))))
  (:`Completed`
    (if (`self.bowDrawn`)
      (bind _hitpoint (`self.LineTraceAiming`))
      (`self.ShootArrow` _hitpoint)
      (goto _label_2 :!via `ReverseFromEnd`))))

(event `EnhancedInput|/Game/Inputs/Actions/IA_DrawBow`
  (params (ActionValue :type Boolean) (ElapsedSeconds :type "Float (double-precision)") (TriggeredSeconds :type "Float (double-precision)") (InputAction :type "InputAction Object Reference" :default "/Game/Inputs/Actions/IA_DrawBow.IA_DrawBow"))
  ; arrow draw animation, and reticle animation
  (:`Triggered`
    ;; if bow is drawn, draw arrow and move reticle bars
    (if (`self.bowDrawn`)
      ;; set reticle and arrow to visible, then invisible
      (`SceneComponent.SetVisibility` (`self.ArrowDecoy`) true false)
      (`SceneComponent.SetVisibility` (`self.reticleBars`) true false)
      (`SceneComponent.SetVisibility` (`self.reticleBars1`) true false)
      (bind (_direction _draw_arrow) (`Timeline|draw arrow` :!label _label_3)
        (:`Update`
          ;; arrow draw animation
          (`SceneComponent.K2_SetRelativeLocation` (`self.ArrowDecoy`) (`KismetMathLibrary.MakeVector` (`KismetMathLibrary.Lerp` (`self.arrowStartDist`) (`self.arrowDrawDist`) _draw_arrow) (`self.distance from player`)) false false)
          ;; reticle animation
          (`SceneComponent.K2_SetRelativeLocation` (`self.reticleBars`) (`KismetMathLibrary.MakeVector` 90.586039 (`KismetMathLibrary.Lerp` -11.35625 -6.368932 _draw_arrow) 0.30677) false false)
          (`SceneComponent.K2_SetRelativeLocation` (`self.reticleBars1`) (`KismetMathLibrary.MakeVector` 90.586039 (`KismetMathLibrary.Lerp` 11.35625 6.368932 _draw_arrow) 0.30677) false false)))))
  (:`Completed`
    (`SceneComponent.SetVisibility` (`self.reticleBars1`) false false)
    (`SceneComponent.SetVisibility` (`self.reticleBars`) false false)
    (`SceneComponent.SetVisibility` (`self.ArrowDecoy`) false false)
    (goto _label_3 :!via `ReverseFromEnd`)))

(fn `AddReticle`
  (bind _returnvalue (`|CreateWidget` "/Game/Blueprints/UI/WB_Reticle.WB_Reticle_C"))
  (`UserWidget.AddToViewport` _returnvalue 0))

(fn `DeleteReticle`
  (bind _returnvalue (`|CreateWidget` "/Game/Blueprints/UI/WB_Reticle.WB_Reticle_C"))
  (`/Engine/EditorBlueprintResources/StandardMacros.IsValid` _returnvalue
    (:`Is Valid`
      (`Widget.RemoveFromParent` _returnvalue))
    (:`Is Not Valid`
      (`KismetSystemLibrary.PrintString` "cant remove"))))

(fn `LineTraceAiming`
  (returns (hitPoint :type "Vector Structure"))
  (bind _camera (`self.Camera`))
  (bind _returnvalue (`SceneComponent.K2_GetComponentLocation` _camera))
  (bind (_outhit _returnvalue_2) (`KismetSystemLibrary.LineTraceSingle` _returnvalue (+ _returnvalue (* (`SceneComponent.GetForwardVector` _camera) (`self.range `))) "TraceTypeQuery1"))
  (if _returnvalue_2
    (bind (_bblockinghit _binitialoverlap _time _distance _location _impactpoint _normal _impactnormal _physmat _hitactor _hitcomponent _hitbonename _bonename _hititem _elementindex _faceindex _tracestart _traceend) (`GameplayStatics.BreakHitResult` _outhit))
    (set `self.impactPoint` _impactpoint)
    (`KismetSystemLibrary.PrintString` "hit")
    (else
      (set `self.impactPoint` _traceend)
      (`KismetSystemLibrary.PrintString` "no hit")))
  (return (`self.impactPoint`)))

(fn `ShootArrow`
  (params (hitPoint :type "Vector Structure"))
  (bind _returnvalue (`SceneComponent.K2_GetComponentLocation` (`self.firePoint`)))
  (bind (_returnvalue_roll _returnvalue_pitch _returnvalue_yaw) (`KismetMathLibrary.BreakRotator` (`KismetMathLibrary.FindLookAtRotation` _returnvalue hitPoint)))
  (`|SpawnActorFromClass` "/Game/Blueprints/BP_ArrowProjectile.BP_ArrowProjectile_C" (`KismetMathLibrary.MakeTransform` _returnvalue (`KismetMathLibrary.MakeRotator` _returnvalue_roll (+ _returnvalue_pitch (`self.randomYRot`)) (+ _returnvalue_yaw (`self.randomXRot`)))) "Undefined" "MultiplyWithRoot" null null))

(fn `UserConstructionScript`)