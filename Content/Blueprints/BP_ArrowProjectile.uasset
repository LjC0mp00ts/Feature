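; BP_ArrowProjectile is an arrow projectile actor that flies with a ProjectileMovement component and destroys itself after a configurable timer.
; When its Box overlaps an actor implementing BPI_Hittable, it sends that actor OnArrowHitMessage with itself, then hides the Trail after a short delay.
; A StopArrowMovement function halts a given arrow's movement and zeroes its gravity, though this Blueprint's own graphs never call it.
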(event `self.ReceiveBeginPlay`
  ; disappears after a time
  (`KismetSystemLibrary.Delay` (`self.TimerToDisappear`))
  (`self.K2_DestroyActor`))

(event `self.Box.OnComponentBeginOverlap`
  (params (OverlappedComponent :type "PrimitiveComponent Object Reference") (OtherActor :type "Actor Object Reference") (OtherComp :type "PrimitiveComponent Object Reference") (OtherBodyIndex :type Integer) (bFromSweep :type Boolean) (SweepResult :type "HitResult Structure (by ref)"))
  ; arrow interface
  (if (`KismetSystemLibrary.DoesImplementInterface` OtherActor "/Game/Blueprints/Interfaces/BPI_Hittable.BPI_Hittable_C")
    (message `/Game/Blueprints/Interfaces/BPI_Hittable.OnArrowHit` OtherActor self)
    (`KismetSystemLibrary.Delay` 0.7)
    (`SceneComponent.SetVisibility` (`self.trail`) false false)))

(fn `StopArrowMovement`
  (params (Arrow :type "/Game/Blueprints/BP_ArrowProjectile Object Reference"))
  (bind _projectilemovement (`/Game/Blueprints/BP_ArrowProjectile.ProjectileMovement` Arrow))
  (`MovementComponent.StopMovementImmediately` _projectilemovement)
  (set `ProjectileMovementComponent.ProjectileGravityScale` 0.0 _projectilemovement))

(fn `UserConstructionScript`)