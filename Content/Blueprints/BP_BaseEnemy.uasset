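; BP_BaseEnemy is an enemy actor that moves along a simple path and takes damage from arrows.
; The construction script adds relative start and end control points to its InterpToMovement component.
; An arrow hit stops the arrow, attaches it to the enemy mesh and damages the health component.
; On death, it destroys every BP_ArrowProjectile in the level, not just attached ones, then itself.
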(event `/Game/Blueprints/Interfaces/BPI_Hittable.OnArrowHit`
  (params (Arrow :type "/Game/Blueprints/BP_ArrowProjectile Object Reference"))
  ; when hit enemy
  ;; stops arrow and attaches to enemy
  (`/Game/Blueprints/BP_ArrowProjectile.StopArrowMovement` Arrow Arrow)
  (`self.K2_AttachToComponent` Arrow (`self.enemy mesh`) "None" "KeepWorld" "KeepWorld" "KeepWorld" true)
  ;; damage
  (`/Game/Blueprints/AC_HealthComponent.TakeDamage` (`self.AC_HealthComponent`) (`self.Amt Damage`)))

(event `self.AC_HealthComponent.OnDeath`
  (bind _outactors (`GameplayStatics.GetAllActorsOfClass` "/Game/Blueprints/BP_ArrowProjectile.BP_ArrowProjectile_C"))
  (`self.K2_DestroyActor` _outactors)
  (`self.K2_DestroyActor`))

(fn `UserConstructionScript`
  (bind _interptomovement (`self.InterpToMovement`))
  ; basic movement
  (`InterpToMovementComponent.AddControlPointPosition` _interptomovement (`self.startLocation`) true)
  (`InterpToMovementComponent.AddControlPointPosition` _interptomovement (`self.endLocation`) true))